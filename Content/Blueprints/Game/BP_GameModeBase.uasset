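; Game mode that drives quests and plays the ending cinematic when one completes.
; Tick executes each quest in QuestArray and pushes its description to the overlay widget.
; On completion it plays the EndMaster sequence, clears the array and removes the overlay.
; Setup of the overlay and state-based C4 quest is disconnected, so this graph never populates either.
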(event EventBeginPlay)

(event EventTick
  (params (DeltaSeconds :type Float%20%28single-precision%29))
  (bind _questarray (Variables|Default|GetQuestArray))
  (bind _questarray_2 (Variables|Default|GetQuestArray))
  (if (not (< (Utilities|Array|Length _questarray_2) 1))
    (for _array_element _questarray_2
      (Class|BTSQuest|Execute _array_element)
      (Utilities|FlowControl|Sequence
        (:then_0
          (if (Class|BTSQuest|GetIsCompleted _array_element)
            (bind _returnvalue (Sequencer|Player|CreateLevelSequencePlayer "/Game/Cinematics/EndMaster.EndMaster"))
            (Sequencer|Player|Play _returnvalue :!class /Script/MovieScene.MovieSceneSequencePlayer)
            (Utilities|Array|Clear _questarray)
            (Utilities|Array|Resize _questarray 0)
            (Widget|RemovefromParent (Variables|Default|GetWBP_Overlay))))
        (:then_1
          (Default|SetQuestText (Variables|Default|GetWBP_Overlay) (Class|BTSQuest|GetQuestDescription _array_element)))))))

(fn ConstructionScript)